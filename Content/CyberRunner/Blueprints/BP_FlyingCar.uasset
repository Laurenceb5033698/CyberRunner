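; BP_FlyingCar is a flying car obstacle that either bounces or crashes the player, depending on which box collider is hit.
; On BeginPlay it binds overlap events to both colliders, though the handler names are swapped relative to their behavior.
; BounceBoxCollider overlaps call Bounced on the JumpCharacter with BoostScalar, while CrashBoxCollider overlaps call PlayerCrashed.
; The car has no movement logic in these graphs, and Tick is disabled.
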(event Custom|OnComponentBeginOverlap_Bounce
  (params (OverlappedComponent :type Primitive%20Component%20Object%20Reference) (OtherActor :type Actor%20Object%20Reference) (OtherComp :type Primitive%20Component%20Object%20Reference) (OtherBodyIndex :type Integer) (bFromSweep :type Boolean) (SweepResult :type Hit%20Result%20Structure%20%28by%20ref%29))
  ;[0.25 0.25 0.25] Actor Collided with Crash Collier
  (if (== OverlappedComponent (Variables|Default|GetCrashBoxCollider))
    (CallFunction|CrashPlayer OtherActor)))

(event Custom|OnComponentBeginOverlap_Crash
  (params (OverlappedComponent :type Primitive%20Component%20Object%20Reference) (OtherActor :type Actor%20Object%20Reference) (OtherComp :type Primitive%20Component%20Object%20Reference) (OtherBodyIndex :type Integer) (bFromSweep :type Boolean) (SweepResult :type Hit%20Result%20Structure%20%28by%20ref%29))
  ;[0.25 0.25 0.25] Actor Collided with bounce collider
  (if (== OverlappedComponent (Variables|Default|GetBounceBoxCollider))
    (CallFunction|BouncePlayer OtherActor)))

(event EventBeginPlay
  (Utilities|FlowControl|Sequence
    (:then_0
      ;[0.25 0.25 0.25] Actor Collided with bounce collider
      (Collision|AssignOnComponentBeginOverlap (Variables|Default|GetBounceBoxCollider) (delegate Custom|OnComponentBeginOverlap_Crash)))
    (:then_1
      ;[0.25 0.25 0.25] Actor Collided with Crash Collier
      (Collision|AssignOnComponentBeginOverlap (Variables|Default|GetCrashBoxCollider) (delegate Custom|OnComponentBeginOverlap_Bounce)))))

(event EventTick
  (params (DeltaSeconds :type Float%20%28single-precision%29)))

(fn ConstructionScript)

(fn BouncePlayer
  (params (Actor :type Actor%20Object%20Reference))
  (bind _asjump_character (Utilities|Casting|CastToJumpCharacter Actor))
  (Default|Bounced _asjump_character (Variables|Default|GetBoostScalar)))

(fn CrashPlayer
  (params (Actor :type Actor%20Object%20Reference))
  (bind _asjump_character (Utilities|Casting|CastToJumpCharacter Actor))
  (Default|PlayerCrashed _asjump_character))