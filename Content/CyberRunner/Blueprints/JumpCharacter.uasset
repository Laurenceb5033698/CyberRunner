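; JumpCharacter is the auto-running player character in CyberRunner, constantly moving along +X until it crashes.
; Jumps use timeline-driven gravity scale, with early release cutting upward velocity.
; Bounce pad launches gain extra power from a jump pressed within short timing windows before or after the bounce.
; Crashes, low falls or reset input destroy the pawn, notifying GM_GameMode of the death and requesting a respawn.
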(event Custom|PlayerCrashed
  (Development|PrintString "Jmp: Player Crashed" true false "(R=1.000000,G=0.666667,B=0.000000,A=1.000000)")
  ;[0.25 0.25 0.25] Halt forward movement and knockback
  (Variables|Character|SetHasCrashed true)
  (Character|LaunchCharacter "-30.000000, 0,-1.000000" true true)
  (Collision|SetCollisionEnabled (Variables|Character|GetMesh) "NoCollision")
  ;[0.25 0.25 0.25] Restart after brief delay
  (Utilities|FlowControl|Delay 1.0)
  (CallFunction|CallRestartPlayer))

(event Custom|Bounced
  (params (Bounce%20Power :type Float%20%28double-precision%29))
  (bind _launchvelocity (Variables|Character|GetLaunchVelocity))
  (Development|PrintString "Jmp: Player Bounced" true false "(R=0.391056,G=1.000000,B=0.000000,A=1.000000)")
  ;[0.3125 0.3125 0.3125] jump pad object caused a bounce
  (if (not (Variables|Character|GetHasCrashed))
    (if (Variables|Character|GettryBounceBoost)
      (Character|LaunchCharacter (* _launchvelocity Bounce%20Power) false true)
      (else
        (Character|LaunchCharacter _launchvelocity false true)))
    (Variables|Character|SetOnBounce true)
    (Utilities|FlowControl|Delay 0.2)
    (Variables|Character|SetOnBounce false)))

(event EventBeginPlay
  (Variables|Character|SetDefaultGravityScale (Variables|/Script/Engine.CharacterMovementComponent|GetGravityScale (Variables|Character|GetCharacterMovement))))

(event Collision|EventActorBeginOverlap
  (params (OtherActor :type Actor%20Object%20Reference)))

(event EventTick
  (params (DeltaSeconds :type Float%20%28single-precision%29))
  (if (not (Variables|Character|GetHasCrashed))
    (Pawn|Input|AddMovementInput "1.000000, 0, 0" 2.0 false)
    ;[0.25 0.25 0.25] player Dies below z height
    (if (< (.z (.location (Transformation|GetActorTransform))) 1e+03)
      (CallFunction|CallRestartPlayer))))

(event EventDestroyed
  ;[0.25 0.25 0.25] Bind event to call GameMode: playerDied
  (bind _asgm_game_mode (Utilities|Casting|CastToGM_GameMode (Game|GetGameMode)))
  (Default|CallOnPlayerDied _asgm_game_mode self))

(event Input|ActionEvents|InputActionJump
  (params (Key :type Key%20Structure :default "None"))
  (bind _charactermovement (Variables|Character|GetCharacterMovement))
  (bind _charactermovement_2 (Variables|Character|GetCharacterMovement))
  (bind _charactermovement_3 (Variables|Character|GetCharacterMovement))
  (:Pressed
    (if (not (Variables|Character|GetHasCrashed))
      (if (Character|CanJump)
        ;[0.25 0.25 0.25] apply jump vel until jump max time or jump key released
        (Character|Jump)
        (bind _newtrack_0 (Timeline|Gravity%20Scale%20onjump PlayFromStart)
          (:Update
            (Variables|/Script/Engine.CharacterMovementComponent|SetGravityScale _charactermovement_3 _newtrack_0))
          (:Finished
            (Variables|/Script/Engine.CharacterMovementComponent|SetGravityScale _charactermovement_3 (Variables|Character|GetDefaultGravityScale) :!label _label)))
        (elif (AI|Components|NavMovement|IsFalling (Variables|Character|GetCharacterMovement))
          ;[0.25 0.25 0.25] set bounce boost and queue unset
          (Variables|Character|SettryBounceBoost true)
          (Utilities|FlowControl|Sequence
            (:then_0
              ;[0.25 0.25 0.25] in air after a jump, land on bounce pad, press jump again to get extra height
              (if (Variables|Character|GetOnBounce) :!label _label_2
                (Variables|Character|SetOnBounce false)
                (Character|LaunchCharacter "0, 0,500.000000" false false)
                (bind _after_bounce_gravity (Timeline|Gravity%20Scale%20After%20Bounce PlayFromStart)
                  (:Update
                    (Variables|/Script/Engine.CharacterMovementComponent|SetGravityScale _charactermovement _after_bounce_gravity))
                  (:Finished
                    (Variables|/Script/Engine.CharacterMovementComponent|SetGravityScale _charactermovement (Variables|Character|GetDefaultGravityScale))))))
            (:then_1
              (Utilities|FlowControl|Delay 0.2)
              (Variables|Character|SettryBounceBoost false)))
          (else
            (goto _label_2))))))
  (:Released
    (Character|StopJumping)
    ;[0.25 0.25 0.25] reduce upwards velocity
    (if (<= (.z (Variables|/Script/Engine.MovementComponent|GetVelocity _charactermovement_2)) 0.0)
      (goto _label)
      (else
        (Variables|/Script/Engine.MovementComponent|SetVelocity _charactermovement_2 (Math|Vector|MakeVector (.x (Variables|/Script/Engine.MovementComponent|GetVelocity _charactermovement_2)) (.y (Variables|/Script/Engine.MovementComponent|GetVelocity _charactermovement_2)) (* (.z (Variables|/Script/Engine.MovementComponent|GetVelocity _charactermovement_2)) 0.7)))
        (goto _label)))))

(event Input|ActionEvents|InputActionResetLevel
  (params (Key :type Key%20Structure :default "None"))
  ;[0.25 0.25 0.25] Input (hotkey) to reset player
  (:Pressed
    (CallFunction|CallRestartPlayer)))

(fn ConstructionScript)

(fn CallRestartPlayer
  (LocalVariables|SetControllerRef (Pawn|GetController))
  (Actor|DestroyActor)
  (bind _asgm_game_mode (Utilities|Casting|CastToGM_GameMode (Game|GetGameMode)))
  (Class|GameModeBase|RestartPlayer _asgm_game_mode (LocalVariables|GetControllerRef)))